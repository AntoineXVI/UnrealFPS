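; BP_Doorgate is a door gate that opens after enough items have been collected.
; Each Collectitem call increments a counter and, once it reaches MaxItemsCollectable, fires OpenDoor through a DoOnce.
; OpenDoor plays the Open timeline, whose DoorP track sets the Door component's relative Z while X and Y are held at zero.
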(event Custom|OpenDoor
  (bind _doorp (Timeline|Open Play)
    (:Update
      (Transformation|SetRelativeLocation (Variables|Default|GetDoor) (Math|Vector|MakeVector 0.0 0.0 _doorp) false false))))

(event Custom|Collect%20item
  (Math|Integer|IncrementInt (Variables|Default|GetcurrentItemsCollected)
    (:%20%20
      (if (>= (Variables|Default|GetcurrentItemsCollected) (Variables|Default|GetmaxItemsCollectable))
        (Utilities|FlowControl|DoOnce false
          (:Completed
            (CallFunction|OpenDoor)))))))

(fn ConstructionScript)